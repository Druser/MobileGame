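; Health potion pickup actor that spins in place and is collected on overlap.
; Any overlap destroys it, then the increment of the potion count stored on ThirdPersonGameMode runs, printing the total and playing a 2D pickup sound.
; The character cast checks player 0 rather than the overlapping actor, and the spin is a fixed yaw step per Tick, independent of frame time.
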(event `self.ReceiveActorBeginOverlap`
  (params (OtherActor :type "Actor Object Reference"))
  (`self.K2_DestroyActor`)
  (cast `/Game/Blueprints/ThirdPersonBP/Blueprints/ThirdPersonCharacter` (`GameplayStatics.GetPlayerCharacter` 0))
  (bind _asthird_person_game_mode (cast `/Game/Blueprints/ThirdPersonBP/Blueprints/ThirdPersonGameMode` (`GameplayStatics.GetGameMode`)))
  (bind _result (`/Engine/EditorBlueprintResources/StandardMacros.IncrementInt` (`/Game/Blueprints/ThirdPersonBP/Blueprints/ThirdPersonGameMode.HealthPotionOwned` _asthird_person_game_mode))
    (:`  `
      (bind _output_get (set `/Game/Blueprints/ThirdPersonBP/Blueprints/ThirdPersonGameMode.HealthPotionOwned` _result _asthird_person_game_mode))
      (`KismetSystemLibrary.PrintString` (`KismetStringLibrary.Concat_StrStr` "Health Potions:" (`KismetStringLibrary.Conv_IntToString` _output_get)))
      (`GameplayStatics.PlaySound2D` "/Game/Assets/Sounds/PickUp.PickUp" 1.0 1.0 0.0 null null))))

(event `self.ReceiveTick`
  (params (DeltaSeconds :type "Float (single-precision)"))
  (`self.K2_AddActorLocalRotation` (`KismetMathLibrary.MakeRotator` 0.0 0.0 3.0)))

(fn `UserConstructionScript`)